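; Actor Blueprint for the RoleShow map that provides camera and post-process helpers, with empty event graph and construction script.
; GetModuleName binds it to the script module Ikun/Maps/RoleShow/LevelVision, following the UnLua convention.
; SetPPSettingFromMat replaces a post-process component's settings with the given dynamic material as a full-weight blendable.
; AAA switches the first player controller's view to a CameraActor found in the level.
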(event EventBeginPlay)

(event Collision|EventActorBeginOverlap
  (params (OtherActor :type Actor%20Object%20Reference)))

(event EventTick
  (params (DeltaSeconds :type Float%20%28single-precision%29)))

(fn ConstructionScript)

(fn SetPPSettingfromMat
  (params (DynMat :type Material%20Instance%20Dynamic%20Object%20Reference) (PPComp :type Post%20Process%20Component%20Object%20Reference))
  (Variables|/Script/Engine.PostProcessComponent|SetSettings PPComp (Utilities|Struct|MakePostProcessSettings (Utilities|Struct|MakeWeightedBlendables (Utilities|Array|MakeArray (Utilities|Struct|MakeWeightedBlendable 1.0 DynMat))))))

(fn AAA
  (bind _returnvalue (Actor|GetActorOfClass "/Script/Engine.CameraActor"))
  (Game|Player|SetViewTargetwithBlend (Game|GetPlayerController 0) _returnvalue 0.0 "VTBlend_Linear" 0.0 false))

(fn GetModuleName
  (return "Ikun/Maps/RoleShow/LevelVision"))