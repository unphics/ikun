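; Site registration component that pushes a site's identity to its site editor widget.
; UpdateSiteInfo casts its widget to UI_SiteEditor and sets the site name and ID; the location ID setter is left unconnected.
; GetModuleName returns a script module path, which points to an UnLua-style binding for logic outside the Blueprint.
; BeginPlay and Tick are unused.
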(event EventBeginPlay)

(event EventTick
  (params (DeltaSeconds :type Float%20%28single-precision%29)))

(fn UpdateSiteInfo
  (bind _asui_site_editor (Utilities|Casting|CastToUI_SiteEditor (UserInterface|GetWidget self)))
  (Default|SetSiteName _asui_site_editor (Variables|Editor|GetSiteName))
  (Default|SetSiteId _asui_site_editor (Variables|Editor|GetSiteId)))

(fn GetModuleName
  (return "Ikun/Blueprint/Comp/BP_SiteRegisterComp"))