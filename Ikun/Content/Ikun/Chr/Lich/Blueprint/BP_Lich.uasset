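; Lich character Blueprint that acts mostly as a shell bound to the script module Ikun.Chr.Lich.BP_Lich through GetModuleName, an UnLua-style binding.
; BeginPlay only calls the parent, and SetLichColor is an empty event, with leftover dynamic-material nodes left unconnected.
; Sphere runs a debug-drawn multi-sphere Visibility trace around the actor and returns the hits, with no caller in this graph.
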(event Custom|SetLichColor
  (params (Color :type Linear%20Color%20Structure)))

(event EventBeginPlay
  (|CallParentFunction))

(event Collision|EventActorBeginOverlap
  (params (OtherActor :type Actor%20Object%20Reference)))

(event EventTick
  (params (DeltaSeconds :type Float%20%28single-precision%29)))

(fn ConstructionScript)

(fn GetModuleName
  (return "Ikun.Chr.Lich.BP_Lich"))

(fn Sphere
  (bind _returnvalue (Transformation|GetActorLocation))
  (bind _outhits (Collision|MultiSphereTraceByChannel _returnvalue _returnvalue 1e+03 "TraceTypeQuery1" false 0 "ForDuration"))
  (return _outhits))